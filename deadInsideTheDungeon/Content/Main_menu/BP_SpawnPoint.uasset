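; BP_SpawnPoint is a spawner that populates its Bound volume with BP_EnemyGuard characters.
; BeginPlay spawns SpawnAmount guards, then a looping timer adds one whenever ActivePawns holds fewer.
; Each spawn uses random bounds points for a debug-drawn downward trace against WorldStatic, placing the guard above the hit location.
; Guards receive an AI_EnemyGuard controller and a reference to this spawner, and are added to ActivePawns.
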(event EventBeginPlay
  (for _index (range 1 (Variables|Default|GetSpawn%20Amount))
    (CallFunction|SpawnCharacter))
  (Utilities|Time|SetTimerbyFunctionName 0 "ReSpawnCharacter" (Variables|Default|GetTimeToRespawn) true))

(fn ConstructionScript)

(fn SpawnCharacter
  (bind _bound (Variables|Default|GetBound))
  (bind (_origin _boxextent) (Collision|GetComponentBounds _bound))
  (bind _returnvalue (Math|Random|RandomPointinBoundingBox _origin _boxextent))
  (bind (_x _y _z) (Math|Vector|BreakVector _returnvalue))
  (bind _returnvalue_2 (+ _z 1e+04))
  (bind _returnvalue_3 (Math|Vector|MakeVector _x _y _returnvalue_2))
  (bind _outhit (Collision|LineTraceForObjects _returnvalue_3 (+ _returnvalue_3 (* (* (Transformation|GetActorUpVector) -1) 1.5e+04)) (Utilities|Array|MakeArray "ObjectTypeQuery1") false 0 "ForDuration"))
  (bind _returnvalue_4 (Game|SpawnActorfromClass "/Game/ThirdPersonBP/Blueprints/BP_EnemyGuard.BP_EnemyGuard_C" (Math|Transform|MakeTransform (Math|Vector|MakeVector (.X (Math|Vector|BreakVector (.Location (Collision|BreakHitResult _outhit)))) (.Y (Math|Vector|BreakVector (.Location (Collision|BreakHitResult _outhit)))) (+ (.Z (Math|Vector|BreakVector (.Location (Collision|BreakHitResult _outhit)))) 1e+02)) (Math|Rotator|MakeRotator 0.0 0.0 (Math|Random|RandomFloat))) "AdjustIfPossibleButAlwaysSpawn" 0 0))
  (Variables|/Script/Engine.Pawn|SetAIControllerClass _returnvalue_4 "/Game/Main_menu/AI/AI_EnemyGuard.AI_EnemyGuard_C")
  (Pawn|SpawnDefaultController _returnvalue_4)
  (Variables|/Game/ThirdPersonBP/Blueprints/BP_EnemyGuard.BP_EnemyGuard_C|SetSpawnPoint _returnvalue_4 self)
  (Utilities|Array|Add (Variables|Default|GetActivePawns) _returnvalue_4))

(fn ReSpawnCharacter
  (if (< (Utilities|Array|Length (Variables|Default|GetActivePawns)) (Variables|Default|GetSpawn%20Amount))
    (CallFunction|SpawnCharacter)))