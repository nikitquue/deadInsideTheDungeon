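; BP_Player is the player character Blueprint for DeadInside, exposing walk speed and handling death.
; Helper functions set and read the character movement's max walk speed or return a self reference.
; Death detaches the pawn from its controller pending destroy, stops movement, clears widgets and blends the view over to a DeathCam child actor.
; It then shows the UI_Death widget with UI-only input and a hidden cursor.
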(event Custom|Death
  (bind _returnvalue (Game|GetPlayerController 0))
  (Class|Pawn|DetachfromControllerPendingDestroy (Game|Player|GetPlayerPawn 0))
  (Components|Movement|StopMovementImmediately (Variables|Character|GetCharacterMovement))
  (Viewport|RemoveAllWidgets)
  (Game|Player|SetViewTargetwithBlend (Game|GetPlayerController 0) (Variables|/Script/Engine.ChildActorComponent|GetChildActor (Variables|Default|GetDeathCam)) 5.0 "VTBlend_Linear" 2.0 false)
  (bind _returnvalue_2 (UserInterface|CreateWidget "/Game/DeadInside/Widget/UI_Death.UI_Death_C" (Game|GetPlayerController 0)))
  (UserInterface|Viewport|AddtoViewport _returnvalue_2 0)
  (Input|SetInputModeUIOnly _returnvalue _returnvalue_2 "DoNotLock")
  (Variables|/Script/Engine.PlayerController|SetbShowMouseCursor _returnvalue false))

(event EventSetPlayerSpeed
  (params (Max%20Walk%20Speed :type Float%20%28single-precision%29))
  (Variables|/Script/Engine.CharacterMovementComponent|SetMaxWalkSpeed (Variables|Character|GetCharacterMovement) Max%20Walk%20Speed))

(fn ConstructionScript)

(fn GetPlayerSpeed
  (return (Variables|/Script/Engine.CharacterMovementComponent|GetMaxWalkSpeed (Variables|Character|GetCharacterMovement))))

(fn PlayerRef
  (return self))