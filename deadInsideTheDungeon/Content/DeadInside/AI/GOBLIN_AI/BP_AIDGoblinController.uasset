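; AI controller for the goblin enemy that turns perception updates into target and noise reactions.
; On possess it caches the pawn's enemy reference, then loops through each updated actor's last sensed stimuli.
; Noise-tagged stimuli pass their location to HeardNoise, while other stimuli count as sight and set the player as target.
; Lost sight starts a retriggerable delay before rechecking the stimulus and clearing or setting the target.
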(event OnPerceptionUpdated(AIPerception)
  (params (UpdatedActors :type Array%20of%20Actor%20Object%20References))
  (for _array_element UpdatedActors
    (bind _info (Class|AIPerceptionComponent|GetActorsPerception (Variables|Default|GetAIPerception) _array_element))
    (for _array_element_2 (.lastsensedstimuli _info)
      (bind _char_ref (Class|BPIPlayer|PlayerRef(Message) (.target _info)))
      (if (Utilities|Name|Equal(Name) (.Tag (Utilities|Struct|BreakAIStimulus _array_element_2)) "Noise")
        (Default|HeardNoise (Variables|Default|GetBP%20Enemy%20Ref) (.StimulusLocation (Utilities|Struct|BreakAIStimulus _array_element_2)))
        (else
          ;[1 1 1] Sight
          (if (.bSuccessfullySensed (Utilities|Struct|BreakAIStimulus _array_element_2))
            (Utilities|IsValid _char_ref :!label _label
              (:Is%20Valid
                (Default|SetNewTarget (Variables|Default|GetBP%20Enemy%20Ref) _char_ref (.bSuccessfullySensed (Utilities|Struct|BreakAIStimulus _array_element_2)) (.StimulusLocation (Utilities|Struct|BreakAIStimulus _array_element_2)))))
            (else
              (Utilities|FlowControl|RetriggerableDelay 1e+01)
              (if (.bSuccessfullySensed (Utilities|Struct|BreakAIStimulus _array_element_2))
                (goto _label)
                (else
                  (Utilities|IsValid _char_ref
                    (:Is%20Valid
                      (Default|ClearTarget (Variables|Default|GetBP%20Enemy%20Ref)))))))))))))

(event EventBeginPlay)

(event EventTick
  (params (DeltaSeconds :type Float%20%28single-precision%29)))

(event EventPossess
  (params (PossessedPawn :type Pawn%20Object%20Reference))
  ;[1 1 1] The same as OnBeginPlay
  (bind _bp_enemy_ref (Class|BPIGoblinBase|EnemyRef(Message) PossessedPawn))
  (Variables|Default|SetBP%20Enemy%20Ref _bp_enemy_ref))

(fn ConstructionScript)