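; Base goblin enemy character that chases a sensed target, investigates noises, takes damage and dies.
; Sensing events set a target and start a looping timer that re-reads its location and moves toward it via AIMoveTo; clearing stops the timer.
; Damage drains armor before health, updating debug text renders, and death halts movement and despawns after a delay.
; Hit reactions check direction but play the same montage for front and side hits.
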(event Custom|Set%20New%20Target
  (params (Target :type Actor%20Object%20Reference) (Sensed :type Boolean) (LastSeenLocation :type Vector))
  ;[1 1 1] Set New Target
  (Variables|Default|GetTarget
    (:then)
    (:else
      (bind _output_get (Variables|Default|SetTarget Target))
      (if Sensed
        (Variables|Default|SetTarget%20Location LastSeenLocation)
        (bind _returnvalue (Utilities|Time|SetTimerbyEvent (delegate Custom|Decisions) 0.25 true))
        (Variables|Default|SetFTimerHandle _returnvalue)
        (CallFunction|ChasePlayer)
        (else
          (Variables|Default|SetTarget%20Location LastSeenLocation))))))

(event Custom|Decisions
  ;[1 1 1] Set New Target
  (Utilities|FlowControl|Delay 1.0)
  (bind _target (Variables|Default|GetTarget)
    (:then
      (if (stale Custom|Set%20New%20Target Sensed)
        (Variables|Default|SetTarget%20Location (Transformation|GetActorLocation _target))
        (CallFunction|ChasePlayer)
        (else
          (Variables|Default|SetTarget%20Location (stale Custom|Set%20New%20Target LastSeenLocation)))))
    (:else)))

(event Custom|Clear%20Target
  ;[1 1 1] Clear Target
  (bind _target (Variables|Default|GetTarget)
    (:then
      (Utilities|Time|ClearandInvalidateTimerbyHandle (Variables|Default|GetFTimerHandle))
      (Transformation|SetActorRotation (Math|Rotator|FindLookatRotation (Transformation|GetActorLocation) (Transformation|GetActorLocation _target)))
      (Utilities|FlowControl|Delay 1.0)
      (Variables|Default|SetTarget 0)
      (CallFunction|StayIdle))
    (:else)))

(event Custom|Chase%20Player
  ;[1 1 1] Chase PLayer
  (Variables|Default|GetTarget
    (:then
      (AI|AIMoveTo self (Variables|Default|GetTarget%20Location) 0 1.5e+02 false))
    (:else)))

(event Custom|Stay%20Idle
  ;[1 1 1] Stay Idle
  (Variables|Default|GetTarget
    (:then
      (AI|AIMoveTo self (Variables|Default|GetTarget%20Location) 0 5.0 true))
    (:else)))

(event Custom|Heard%20Noise
  (params (Noise%20Location :type Vector))
  ;[1 1 1] Heard Noise
  (Variables|Default|GetTarget
    (:then)
    (:else
      (AI|AIMoveTo self Noise%20Location 0 5.0 true))))

(event Custom|Enemy%20Dead
  ;[1 1 1] Dead
  (Utilities|FlowControl|DoOnce false
    (:Completed
      (Actor|SetLifeSpan 1e+01))))

(event Custom|PLay%20Goblin%20Hit
  (params (Hit%20Direction :type Float%20%28single-precision%29))
  ;[1 1 1] Goblin Hit
  (if (Math|Float|InRange(Float) Hit%20Direction -45.0 45.0)
    (Animation|Montage|PlayMontage (Variables|Character|GetMesh) "/Game/DeadInside/AI/GOBLIN_AI/AnimationMontages/Goblin_Hit.Goblin_Hit"
      (:then
        (Development|PrintString "Front")))
    (elif (Math|Float|InRange(Float) Hit%20Direction -135.0 -45.0 true false)
      (Animation|Montage|PlayMontage (Variables|Character|GetMesh) "/Game/DeadInside/AI/GOBLIN_AI/AnimationMontages/Goblin_Hit.Goblin_Hit"
        (:then
          (Development|PrintString "Front")))
      (elif (Math|Float|InRange(Float) Hit%20Direction 45.0 135.0 false)
        (Animation|Montage|PlayMontage (Variables|Character|GetMesh) "/Game/DeadInside/AI/GOBLIN_AI/AnimationMontages/Goblin_Hit.Goblin_Hit"
          (:then
            (Development|PrintString "Front")))))))

(event EventBeginPlay
  (bind _enemy_info (Variables|Default|GetEnemy%20Info))
  (bind (_maxhealth _currenthealth _maxarmor _currentarmor) (Utilities|Struct|BreakPlayerInfo _enemy_info))
  (|CallParentFunction)
  (Rendering|Components|TextRender|SetText (Variables|Default|GetTextRender) (Utilities|Text|ToText(Float) _currentarmor "HalfToEven"))
  (Rendering|Components|TextRender|SetText (Variables|Default|GetTextRender1) (Utilities|Text|ToText(Float) _currenthealth "HalfToEven")))

(event Collision|EventActorBeginOverlap
  (params (OtherActor :type Actor%20Object%20Reference))
  (|CallParentFunction OtherActor) ; This node is disabled and will not be called.\nDrag off pins to build functionality.
)

(event EventTick
  (params (DeltaSeconds :type Float%20%28single-precision%29))
  (|CallParentFunction DeltaSeconds) ; This node is disabled and will not be called.\nDrag off pins to build functionality.
)

(fn ConstructionScript
  (|CallParentFunction))

(fn FDamageDealt
  (params (Damage%20Dealt :type Float%20%28single-precision%29))
  (bind _enemy_info (Variables|Default|GetEnemy%20Info))
  (bind _enemy_info_2 (Variables|Default|GetEnemy%20Info))
  (bind (_maxhealth _currenthealth _maxarmor _currentarmor) (Utilities|Struct|BreakPlayerInfo _enemy_info))
  (bind (_maxhealth_2 _currenthealth_2) (Utilities|Struct|BreakPlayerInfo _enemy_info_2))
  (bind _returnvalue (- _currentarmor Damage%20Dealt))
  (bind _returnvalue_2 (- _currenthealth_2 Damage%20Dealt))
  (bind _returnvalue_3 (Math|Float|Clamp(Float) _returnvalue 0.0 _maxarmor))
  (bind _returnvalue_4 (Math|Float|Clamp(Float) _returnvalue_2 0.0 _maxhealth_2))
  (if (<= _currentarmor 0.0)
    (Utilities|Struct|SetmembersinPlayerInfo (Variables|Default|GetEnemy%20Info) _returnvalue_4)
    (Rendering|Components|TextRender|SetText (Variables|Default|GetTextRender1) (Utilities|Text|ToText(Float) _returnvalue_4 "HalfToEven"))
    (if (<= (Utilities|Struct|BreakPlayerInfo (Variables|Default|GetEnemy%20Info)) 0.0)
      (Variables|Default|SetbIsEnemyDead true)
      (Utilities|Time|ClearandInvalidateTimerbyHandle (Variables|Default|GetFTimerHandle))
      (Pawn|Components|CharacterMovement|SetMovementMode (Variables|Character|GetCharacterMovement) "MOVE_None" 0)
      (CallFunction|EnemyDead))
    (else
      (Utilities|Struct|SetmembersinPlayerInfo (Variables|Default|GetEnemy%20Info) _returnvalue_3)
      (Rendering|Components|TextRender|SetText (Variables|Default|GetTextRender) (Utilities|Text|ToText(Float) _returnvalue_3 "HalfToEven")))))

(fn EnemyRef
  (return self))