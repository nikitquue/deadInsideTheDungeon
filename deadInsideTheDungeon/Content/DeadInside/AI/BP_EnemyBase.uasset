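; Base melee enemy character that chases and attacks the player, using spider montages and a socketed sword.
; Externally triggered events set or clear the target or investigate noises; a looping timer refreshes chase movement, leading to attack on arrival.
; A montage notify fires a sphere overlap that damages the player unless blocking.
; Incoming damage depletes armor before health, updates text readouts, and at zero health stops movement and expires the actor.
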(event Custom|Set%20New%20Target
  (params (Target :type Actor%20Object%20Reference) (Sensed :type Boolean) (LastSeenLocation :type Vector))
  ;[1 1 1] Set New Target
  (if (not (Variables|/Game/DeadInside/Character/BP_Player.BP_Player_C|GetbIsPlayerDead (Variables|Default|GetChar%20Ref)))
    (Variables|Default|GetTarget
      (:then)
      (:else
        (Variables|Default|SetTarget Target)
        (if (and (not (Variables|Default|GetbIsEnemyDead)) (not (Variables|Default|GetbAMIsPlaying)))
          (if Sensed
            (Variables|Default|SetTarget%20Location LastSeenLocation)
            (bind _returnvalue (Utilities|Time|SetTimerbyEvent (delegate Custom|Decisions) 0.25 true))
            (Variables|Default|SetFTimerHandle _returnvalue)
            (CallFunction|EquipWeapon)
            (CallFunction|ChasePlayer)))))))

(event Custom|Decisions
  ;[1 1 1] Set New Target
  (bind _target (Variables|Default|GetTarget)
    (:then
      (if (and (not (Variables|/Game/DeadInside/Character/BP_Player.BP_Player_C|GetbIsPlayerDead (Variables|Default|GetChar%20Ref))) (stale Custom|Set%20New%20Target Sensed))
        (Variables|Default|SetTarget%20Location (Transformation|GetActorLocation _target))
        (CallFunction|ChasePlayer)))
    (:else)))

(event Custom|Play%20Hit%20Montage
  (params (Hit%20Direction :type Float%20%28single-precision%29))
  ;[1 1 1] Play Hit Montage According to direction
  (if (Math|Float|InRange(Float) Hit%20Direction -45.0 45.0)
    (Animation|Montage|PlayMontage (Variables|Character|GetMesh) "/Game/Animations/Boss/AM_Spider_Hit.AM_Spider_Hit")
    (elif (Math|Float|InRange(Float) Hit%20Direction -135.0 -45.0 true false)
      (Animation|Montage|PlayMontage (Variables|Character|GetMesh) "/Game/Animations/Boss/AM_Spider_Hit.AM_Spider_Hit")
      (elif (Math|Float|InRange(Float) Hit%20Direction 45.0 135.0 false)
        (Animation|Montage|PlayMontage (Variables|Character|GetMesh) "/Game/Animations/Boss/AM_Spider_Hit.AM_Spider_Hit")))))

(event Custom|UnequipWeapon
  ;[1 1 1] Unequip Weapon
  (Transformation|AttachComponentToComponent (Variables|Default|GetSword) (Variables|Character|GetMesh) "WeaponSocket" "SnapToTarget" "SnapToTarget" "SnapToTarget" true))

(event Custom|EquipWeapon
  ;[1 1 1] Equip Weapon
  (Transformation|AttachComponentToComponent (Variables|Default|GetSword) (Variables|Character|GetMesh) "WeaponHolster" "SnapToTarget" "SnapToTarget" "SnapToTarget" true))

(event Custom|Clear%20Target
  ;[1 1 1] Clear Target
  (bind _target (Variables|Default|GetTarget)
    (:then
      (Utilities|Time|ClearandInvalidateTimerbyHandle (Variables|Default|GetFTimerHandle))
      (if (Variables|Default|GetbIsEnemyDead)
        _
        (else
          (Transformation|SetActorRotation (Math|Rotator|FindLookatRotation (Transformation|GetActorLocation) (Transformation|GetActorLocation _target)))))
      (Utilities|FlowControl|Delay 1.0)
      (Variables|Default|SetTarget 0)
      (CallFunction|UnequipWeapon)
      (CallFunction|StayIdle))
    (:else)))

(event Custom|ChasePlayer
  ;[1 1 1] Chase Player
  (if (and (not (Variables|Default|GetbIsEnemyDead)) (not (Variables|Default|GetbAMIsPlaying)))
    (Variables|Default|GetTarget
      (:then
        (AI|AIMoveTo self (Variables|Default|GetTarget%20Location) 0 1.5e+02 false
          (:OnSuccess
            (CallFunction|Attack))))
      (:else))))

(event Custom|Stay%20Idle
  ;[1 1 1] Stay Idle
  (Variables|Default|GetTarget
    (:then
      (AI|AIMoveTo self (Variables|Default|GetTarget%20Location) 0 5.0 true))
    (:else)))

(event Custom|Heard%20Noise
  (params (Noise%20Location :type Vector))
  ;[1 1 1] Heard Noise
  (Variables|Default|GetTarget
    (:then)
    (:else
      (AI|AIMoveTo self Noise%20Location 0 5.0 true))))

(event Custom|Enemy%20Dead
  ;[1 1 1] Dead Enemy
  (Utilities|FlowControl|DoOnce false
    (:Completed
      (Actor|SetLifeSpan 1e+01))))

(event Custom|Attack
  (bind _returnvalue (Transformation|GetActorRotation))
  ;[1 1 1] Attack Montage
  (if (and (not (Variables|Default|GetbIsEnemyDead)) (not (Variables|Default|GetbAMIsPlaying)))
    (Variables|Default|GetTarget
      (:then
        (Transformation|SetActorRotation (Math|Rotator|MakeRotator (.roll _returnvalue) (.pitch _returnvalue) (.yaw (Math|Rotator|FindLookatRotation (Transformation|GetActorLocation) (Transformation|GetActorLocation (Variables|Default|GetTarget))))))
        (Variables|Default|SetbAMIsPlaying true)
        (Animation|Montage|PlayMontage (Variables|Character|GetMesh) "/Game/Animations/Boss/AM_Spider_Melee.AM_Spider_Melee"
          (:OnBlendOut
            (Variables|Default|SetbAMIsPlaying false))
          (:OnNotifyBegin
            (CallFunction|LightAttack))))
      (:else))))

(event Custom|LightAttack
  (bind _self self)
  ;[1 1 1] Light Attack
  (bind (_outactors _returnvalue) (Collision|SphereOverlapActors (+ (Transformation|GetActorLocation _self) (* (Transformation|GetActorForwardVector _self) 1e+02)) 1.5e+02 (Utilities|Array|MakeArray "ObjectTypeQuery3") 0 (Utilities|Array|MakeArray self)))
  (Utilities|FlowControl|Sequence
    (:then_0
      (if _returnvalue
        (for _array_element _outactors
          (Class|BPIPlayer|PlayerRef(Message) _array_element)
          (bind _pc_ref (Class|BPIPC|PCRef(Message) (Game|GetPlayerController 0)))
          (if (Variables|/Game/DeadInside/PlayerController/BP_PlayerController.BP_PlayerController_C|GetbIsBlocking _pc_ref)
            (Default|DamageDealt _pc_ref 0.0)
            (else
              (Default|DamageDealt _pc_ref 5e+01))))))))

(event EventBeginPlay
  (bind _enemy_info (Variables|Default|GetEnemy%20Info))
  (bind (_currenthealth _currentarmor) (Utilities|Struct|BreakPlayerInfo _enemy_info))
  (|CallParentFunction)
  (Rendering|Components|TextRender|SetText (Variables|Default|GetTextRender) (Utilities|Text|ToText(Float) _currentarmor "HalfToEven"))
  (Rendering|Components|TextRender|SetText (Variables|Default|GetTextRender1) (Utilities|Text|ToText(Float) _currenthealth "HalfToEven"))
  (bind _pc_ref (Class|BPIPC|PCRef(Message) (Variables|Default|GetTarget)))
  (Variables|Default|SetPC%20Ref _pc_ref)
  (bind _char_ref (Class|BPIPlayer|PlayerRef(Message) (Game|GetPlayerCharacter 0)))
  (Variables|Default|SetChar%20Ref _char_ref))

(event Collision|EventActorBeginOverlap
  (params (OtherActor :type Actor%20Object%20Reference))
  (|CallParentFunction OtherActor) ; This node is disabled and will not be called.\nDrag off pins to build functionality.
)

(event EventTick
  (params (DeltaSeconds :type Float%20%28single-precision%29))
  (|CallParentFunction DeltaSeconds)
  (if (Variables|/Game/DeadInside/PlayerController/BP_PlayerController.BP_PlayerController_C|GetbIsPlayerDead (Variables|Default|GetPC%20Ref))
    (Utilities|FlowControl|DoOnce false :!label _label
      (:Completed
        (CallFunction|ClearTarget)))
    (else
      (goto _label Reset))))

(fn ConstructionScript
  (|CallParentFunction))

(fn FDamageDealt
  (params (Damage%20Dealt :type Float%20%28single-precision%29))
  (bind _enemy_info (Variables|Default|GetEnemy%20Info))
  (bind _enemy_info_2 (Variables|Default|GetEnemy%20Info))
  (bind (_maxarmor _currentarmor) (Utilities|Struct|BreakPlayerInfo _enemy_info))
  (bind (_maxhealth _currenthealth) (Utilities|Struct|BreakPlayerInfo _enemy_info_2))
  (bind _returnvalue (- _currentarmor Damage%20Dealt))
  (bind _returnvalue_2 (- _currenthealth Damage%20Dealt))
  (bind _returnvalue_3 (Math|Float|Clamp(Float) _returnvalue_2 0.0 _maxhealth))
  (bind _returnvalue_4 (Math|Float|Clamp(Float) _returnvalue 0.0 _maxarmor))
  (Variables|Default|SetbAMIsPlaying false)
  (if (<= _currentarmor 0.0)
    (Rendering|Components|TextRender|SetText (Variables|Default|GetTextRender1) (Utilities|Text|ToText(Float) _returnvalue_3 "HalfToEven"))
    (Utilities|Struct|SetmembersinPlayerInfo (Variables|Default|GetEnemy%20Info) _returnvalue_3)
    (if (<= (Utilities|Struct|BreakPlayerInfo (Variables|Default|GetEnemy%20Info)) 0.0)
      (Variables|Default|SetbIsEnemyDead true)
      (Utilities|Time|ClearandInvalidateTimerbyHandle (Variables|Default|GetFTimerHandle))
      (Pawn|Components|CharacterMovement|SetMovementMode (Variables|Character|GetCharacterMovement) "MOVE_None" 0)
      (CallFunction|EnemyDead))
    (else
      (Rendering|Components|TextRender|SetText (Variables|Default|GetTextRender) (Utilities|Text|ToText(Float) _returnvalue_4 "HalfToEven"))
      (Utilities|Struct|SetmembersinPlayerInfo (Variables|Default|GetEnemy%20Info) _returnvalue_4))))

(fn EnemyRef
  (return self))