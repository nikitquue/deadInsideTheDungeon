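; Base interactable actor that registers itself with the player controller while the player is inside its Box trigger.
; On overlap begin, it confirms the player through a PlayerRef message and passes itself to the controller through InteractRef.
; On overlap end, the same check sends an empty InteractRef to clear it.
; InteractableRef returns the actor itself, and no interaction behaviour is implemented here.
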(event OnComponentBeginOverlap(Box)
  (params (OverlappedComponent :type Primitive%20Component%20Object%20Reference) (OtherActor :type Actor%20Object%20Reference) (OtherComp :type Primitive%20Component%20Object%20Reference) (OtherBodyIndex :type Integer) (bFromSweep :type Boolean) (SweepResult :type Hit%20Result%20Structure%20%28by%20ref%29))
  (bind _char_ref (Class|BPIPlayer|PlayerRef(Message) OtherActor))
  (if (== _char_ref OtherActor)
    (bind _pc_ref (Class|BPIPC|PCRef(Message) (Game|GetPlayerController 0)))
    (Class|BPIPC|InteractRef(Message) _pc_ref self)))

(event OnComponentEndOverlap(Box)
  (params (OverlappedComponent :type Primitive%20Component%20Object%20Reference) (OtherActor :type Actor%20Object%20Reference) (OtherComp :type Primitive%20Component%20Object%20Reference) (OtherBodyIndex :type Integer))
  (bind _char_ref (Class|BPIPlayer|PlayerRef(Message) OtherActor))
  (if (== _char_ref OtherActor)
    (bind _pc_ref (Class|BPIPC|PCRef(Message) (Game|GetPlayerController 0)))
    (Class|BPIPC|InteractRef(Message) _pc_ref)))

(event EventBeginPlay)

(event Collision|EventActorBeginOverlap
  (params (OtherActor :type Actor%20Object%20Reference)))

(event EventTick
  (params (DeltaSeconds :type Float%20%28single-precision%29)))

(fn ConstructionScript)

(fn InteractableRef
  (return self))