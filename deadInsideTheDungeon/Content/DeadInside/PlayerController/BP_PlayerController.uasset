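; Player controller for Dead Inside that turns input into movement, sprint, directional rolls, blocking, montage combos and a noise distraction, and creates the HUD.
; A Tick sphere trace picks interactables, which are routed by pickup type to weapon/shield socket swaps or capped health and potion stocks.
; Attack montage notifies damage the closest enemy in a forward sphere overlap.
; PlayerInfo holds health and armor: damage drains armor first, and drink montages restore either.
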(event Custom|Weapon%20Pickup
  (params (Current%20Interactable%20Ref :type Actor%20Object%20Reference))
  (bind _char_ref (Variables|Character|GetChar%20Ref))
  ;[1 1 1] Weapon Pickup
  (bind _weapon (Variables|Inventory|GetWeapon)
    (:then
      (Variables|Inventory|SetWeaponInHandClass (Utilities|GetClass _weapon))
      (Actor|DestroyActor _weapon)
      (bind _output_get (Variables|Inventory|SetWeapon Current%20Interactable%20Ref))
      (Transformation|AttachComponentToComponent _output_get (Variables|/Script/Engine.Character|GetMesh _char_ref) "WeaponSocket" "SnapToTarget" "SnapToTarget" "SnapToTarget" true)
      (bind _interact_ref (Class|BPIInteract|InteractableRef(Message) _output_get))
      (Collision|SetActorEnableCollision _interact_ref false)
      (Variables|/Game/DeadInside/Interactables/BP_BaseInteractables.BP_BaseInteractables_C|SetRotate _interact_ref false)
      (Game|SpawnActorfromClass (Variables|Inventory|GetWeaponInHandClass) (Math|Transform|MakeTransform (+ (Transformation|GetWorldLocation (Variables|/Script/Engine.Character|GetMesh _char_ref)) (* (Math|Vector|GetForwardVector (Variables|/Script/Engine.Character|GetCapsuleComponent _char_ref)) 1e+01)) "-90.000000,0.000000, 0" "1,1,1") "AdjustIfPossibleButAlwaysSpawn" 0 0))
    (:else
      (bind _output_get_2 (Variables|Inventory|SetWeapon Current%20Interactable%20Ref))
      (Transformation|AttachComponentToComponent _output_get_2 (Variables|/Script/Engine.Character|GetMesh (Variables|Character|GetChar%20Ref)) "WeaponSocket" "SnapToTarget" "SnapToTarget" "SnapToTarget" true)
      (bind _interact_ref_2 (Class|BPIInteract|InteractableRef(Message) _output_get_2))
      (Collision|SetActorEnableCollision _interact_ref_2 false)
      (Variables|/Game/DeadInside/Interactables/BP_BaseInteractables.BP_BaseInteractables_C|SetRotate _interact_ref_2 false))))

(event Custom|Shield%20Pickup
  (params (Current%20Interactable%20Ref :type Actor%20Object%20Reference))
  (bind _char_ref (Variables|Character|GetChar%20Ref))
  ;[1 1 1] Shield Pickup Logic
  (bind _shield (Variables|Inventory|GetShield)
    (:then
      (Variables|Inventory|SetShieldInHandClass (Utilities|GetClass _shield))
      (Actor|DestroyActor _shield)
      (bind _output_get (Variables|Inventory|SetShield Current%20Interactable%20Ref))
      (Transformation|AttachComponentToComponent _output_get (Variables|/Script/Engine.Character|GetMesh _char_ref) "ShieldSocket" "SnapToTarget" "SnapToTarget" "SnapToTarget" true)
      (bind _interact_ref (Class|BPIInteract|InteractableRef(Message) _output_get))
      (Collision|SetActorEnableCollision _interact_ref false)
      (Variables|/Game/DeadInside/Interactables/BP_BaseInteractables.BP_BaseInteractables_C|SetRotate _interact_ref false)
      (Game|SpawnActorfromClass (Variables|Inventory|GetShieldInHandClass) (Math|Transform|MakeTransform (+ (Transformation|GetWorldLocation (Variables|/Script/Engine.Character|GetMesh _char_ref)) (* (Math|Vector|GetForwardVector (Variables|/Script/Engine.Character|GetCapsuleComponent _char_ref)) 1e+01)) "0.000000,0.000000,-90.000000" "1,1,1") "AdjustIfPossibleButAlwaysSpawn" 0 0))
    (:else
      (bind _output_get_2 (Variables|Inventory|SetShield Current%20Interactable%20Ref))
      (Transformation|AttachComponentToComponent _output_get_2 (Variables|/Script/Engine.Character|GetMesh (Variables|Character|GetChar%20Ref)) "ShieldSocket" "SnapToTarget" "SnapToTarget" "SnapToTarget" true)
      (bind _interact_ref_2 (Class|BPIInteract|InteractableRef(Message) _output_get_2))
      (Collision|SetActorEnableCollision _interact_ref_2 false)
      (Variables|/Game/DeadInside/Interactables/BP_BaseInteractables.BP_BaseInteractables_C|SetRotate _interact_ref_2 false))))

(event Custom|Damage%20Closest%20Enemy
  (bind _char_ref (Variables|Character|GetChar%20Ref))
  (bind _char_ref_2 (Variables|Character|GetChar%20Ref))
  ;[1 1 1] Damage
  (bind (_outactors _returnvalue) (Collision|SphereOverlapActors (+ (Transformation|GetActorLocation _char_ref) (* (Transformation|GetActorForwardVector _char_ref) 1e+02)) 1.5e+02 (Utilities|Array|MakeArray "ObjectTypeQuery8") 0 (Utilities|Array|MakeArray (Variables|Character|GetChar%20Ref))))
  (Utilities|FlowControl|Sequence
    (:then_0
      (if _returnvalue
        (for _array_element _outactors
          (bind _bp_enemy_ref (Class|BPIEnemy|EnemyRef(Message) _array_element))
          (if (not (Variables|/Game/DeadInside/AI/BP_EnemyBase.BP_EnemyBase_C|GetbIsEnemyDead _bp_enemy_ref))
            (Variables|Default|GetClosestEnemy
              (:then
                (if (< (Transformation|GetDistanceTo _array_element _char_ref_2) (Transformation|GetDistanceTo (Variables|Default|GetClosestEnemy) _char_ref_2))
                  (Variables|Default|SetClosestEnemy _array_element)))
              (:else
                (Variables|Default|SetClosestEnemy _array_element)))))
        (bind _bp_enemy_ref_2 (Class|BPIEnemy|EnemyRef(Message) (Variables|Default|GetClosestEnemy)))
        (if (not (Variables|/Game/DeadInside/AI/BP_EnemyBase.BP_EnemyBase_C|GetbIsEnemyDead _bp_enemy_ref_2))
          (Default|PlayHitMontage _bp_enemy_ref_2 (.yaw (Math|Rotator|FindLookatRotation (Transformation|GetActorLocation (Variables|Default|GetClosestEnemy)) (Transformation|GetActorLocation (Variables|Character|GetChar%20Ref)))))
          (bind _interact_ref (Class|BPIInteract|InteractableRef(Message) (Variables|Inventory|GetWeapon)))
          (Default|FDamageDealt _bp_enemy_ref_2 (Variables|/Game/DeadInside/Interactables/BP_BaseInteractables.BP_BaseInteractables_C|GetWeaponDamage _interact_ref)))))))

(event Custom|Damage%20Closest%20Goblin
  (bind _char_ref (Variables|Character|GetChar%20Ref))
  (bind _char_ref_2 (Variables|Character|GetChar%20Ref))
  (bind _returnvalue (Transformation|GetActorLocation _char_ref))
  (bind _returnvalue_2 (Transformation|GetActorForwardVector _char_ref))
  (bind _returnvalue_3 (* _returnvalue_2 2.5e+02))
  (bind _returnvalue_4 (+ _returnvalue_3 _returnvalue))
  (bind (_outactors _returnvalue_5) (Collision|SphereOverlapActors _returnvalue_4 2.5e+02 (Utilities|Array|MakeArray "ObjectTypeQuery8") 0 (Utilities|Array|MakeArray (Variables|Character|GetChar%20Ref))))
  (Utilities|FlowControl|Sequence
    (:then_0
      (if _returnvalue_5
        (for _array_element _outactors
          (bind _bp_enemy_ref (Class|BPIGoblinBase|EnemyRef(Message) _array_element))
          (Variables|Default|GetClosestGoblin
            (:then
              (if (< (Transformation|GetDistanceTo _array_element _char_ref_2) (Transformation|GetDistanceTo (Variables|Default|GetClosestGoblin) _char_ref_2))
                (Variables|Default|SetClosestGoblin _array_element)))
            (:else
              (Variables|Default|SetClosestGoblin _array_element)
              (Default|FDamageDealt _bp_enemy_ref 1e+01))))
        (bind _bp_enemy_ref_2 (Class|BPIGoblinBase|EnemyRef(Message) (Variables|Default|GetClosestEnemy)))
        (Default|PLayGoblinHit _bp_enemy_ref_2 (.yaw (Math|Rotator|FindLookatRotation (Transformation|GetActorLocation (Variables|Default|GetClosestEnemy)) (Transformation|GetActorLocation (Variables|Character|GetChar%20Ref)))))
        (Default|FDamageDealt _bp_enemy_ref_2 3e+01)))
    (:then_1
      (Rendering|Debug|DrawDebugSphere _returnvalue_4 2.5e+02 12 "(R=1.000000,G=0.000000,B=0.174811,A=1.000000)" 5.0 1.0))))

(event Custom|Potion%20Pickup
  (params (Current%20Interactable%20Ref :type Actor%20Object%20Reference))
  ;[1 1 1] Health and Potion pickup
  (if (< (Variables|Inventory|GetPotion%20Count) 4)
    (Utilities|Array|Add (Variables|Inventory|GetPotion) Current%20Interactable%20Ref)
    (Actor|DestroyActor Current%20Interactable%20Ref)
    (bind _result (Math|Integer|IncrementInt (Variables|Inventory|GetPotion%20Count))
      (:%20%20
        (Variables|Inventory|SetPotion%20Count _result)))))

(event Custom|Health%20Pickup
  (params (Current%20Interactable%20Ref :type Actor%20Object%20Reference))
  ;[1 1 1] Health and Potion pickup
  (if (< (Variables|Inventory|GetHealth%20Count) 4)
    (Utilities|Array|Add (Variables|Inventory|GetHealth) Current%20Interactable%20Ref)
    (Actor|DestroyActor Current%20Interactable%20Ref)
    (bind _result (Math|Integer|IncrementInt (Variables|Inventory|GetHealth%20Count))
      (:%20%20
        (Variables|Inventory|SetHealth%20Count _result)))))

(event Custom|Basic%20Attack
  ;[1 1 1] Attack
  (bind _weapon (Variables|Inventory|GetWeapon)
    (:then
      (if (and (not (Variables|Boolean|GetbIsAMPlaying)) (not (Variables|Boolean|GetbIsRMPlaying)))
        (bind _interact_ref (Class|BPIInteract|InteractableRef(Message) _weapon))
        (Utilities|IsValid (Utilities|Array|Get(acopy) (Variables|/Game/DeadInside/Interactables/BP_BaseInteractables.BP_BaseInteractables_C|GetSword%20Anims _interact_ref) (Variables|Combat|GetCombo%20Count))
          (:Is%20Valid
            (Variables|Boolean|SetbIsAMPlaying true)
            (Variables|Boolean|SetbIsBlocking false)
            (Animation|Montage|PlayMontage (Variables|/Script/Engine.Character|GetMesh (Variables|Character|GetChar%20Ref)) (Utilities|Array|Get(acopy) (Variables|/Game/DeadInside/Interactables/BP_BaseInteractables.BP_BaseInteractables_C|GetSword%20Anims _interact_ref) (Variables|Combat|GetCombo%20Count))
              (:OnBlendOut
                (Utilities|FlowControl|Sequence
                  (:then_0
                    (if (< (Variables|Combat|GetCombo%20Count) (- (Utilities|Array|Length (Variables|/Game/DeadInside/Interactables/BP_BaseInteractables.BP_BaseInteractables_C|GetSword%20Anims _interact_ref)) 1)) :!label _label
                      (Utilities|FlowControl|Sequence
                        (:then_0
                          (Math|Integer|IncrementInt (Variables|Combat|GetCombo%20Count)
                            (:%20%20
                              (Variables|Boolean|SetbIsAMPlaying false))))
                        (:then_1
                          (Utilities|FlowControl|RetriggerableDelay 0.2)
                          (if (not (Variables|Boolean|GetbIsAMPlaying))
                            (Variables|Combat|SetCombo%20Count 0)
                            (Variables|Boolean|SetbIsAMPlaying false))))
                      (else
                        (Variables|Combat|SetCombo%20Count 0 :!label _label_2)
                        (Variables|Boolean|SetbIsAMPlaying false))))
                  (:then_1
                    (if (Game|Player|IsInputKeyDown "RightMouseButton")
                      (Variables|Boolean|SetbIsBlocking true)
                      (else
                        (Variables|Boolean|SetbIsBlocking false))))))
              (:OnInterrupted
                (goto _label))
              (:OnNotifyBegin
                (CallFunction|DamageClosestEnemy))))
          (:Is%20Not%20Valid
            (goto _label_2)))))
    (:else)))

(event Custom|Roll
  ;[1 1 1] Roll Logic
  (if (not (Variables|Boolean|GetbIsRMPlaying))
    (if (Utilities|RollBackCondition)
      (CallFunction|RollBack)
      (elif (Utilities|RollForwardCondition)
        (CallFunction|RollForward)
        (elif (Utilities|RollRightCondition)
          (CallFunction|RollRight)
          (elif (Utilities|RollLeftCondition)
            (CallFunction|RollLeft)
            (else
              (CallFunction|RollBack))))))))

(event Custom|Roll%20Back
  ;[1 1 1] Roll Back
  (Variables|Boolean|SetbIsRMPlaying true)
  (Animation|Montage|PlayMontage (Variables|/Script/Engine.Character|GetMesh (Variables|Character|GetChar%20Ref)) "/Game/DeadInside/Character/Animations/AM_RollBackN.AM_RollBackN"
    (:OnBlendOut
      (Variables|Boolean|SetbIsRMPlaying false))))

(event Custom|RollForward
  ;[1 1 1] Roll Forward
  (Variables|Boolean|SetbIsRMPlaying true)
  (Animation|Montage|PlayMontage (Variables|/Script/Engine.Character|GetMesh (Variables|Character|GetChar%20Ref)) "/Game/DeadInside/Character/Animations/AM_RollForward.AM_RollForward"
    (:OnBlendOut
      (Variables|Boolean|SetbIsRMPlaying false))))

(event Custom|Roll%20Right
  ;[1 1 1] Roll RIght
  (Variables|Boolean|SetbIsRMPlaying true)
  (Animation|Montage|PlayMontage (Variables|/Script/Engine.Character|GetMesh (Variables|Character|GetChar%20Ref)) "/Game/DeadInside/Character/Animations/AM_RollForward.AM_RollForward"
    (:OnBlendOut
      (Variables|Boolean|SetbIsRMPlaying false))))

(event Custom|Roll%20Left
  ;[1 1 1] Roll Left
  (Variables|Boolean|SetbIsRMPlaying true)
  (Animation|Montage|PlayMontage (Variables|/Script/Engine.Character|GetMesh (Variables|Character|GetChar%20Ref)) "/Game/DeadInside/Character/Animations/AM_RollLeft.AM_RollLeft"
    (:OnBlendOut
      (Variables|Boolean|SetbIsRMPlaying false))))

(event EventInteractRef
  (params (Interact%20Ref :type BP%20Base%20Interactables%20Object%20Reference))
  ;[1 1 1] Interaction Reference
  (Variables|Inventory|SetCurrent%20Interactable Interact%20Ref))

(event EventTick
  (params (DeltaSeconds :type Float%20%28single-precision%29))
  (bind _outlocation (Actor|GetActorEyesViewPoint))
  ;[1 1 1] Event TIck
  (if (> (Utilities|Array|Length (Variables|Inventory|GetInteractablesInRange)) 0)
    (bind (_outhit _returnvalue) (Collision|SphereTraceForObjects _outlocation (* _outlocation (* (Math|Vector|GetForwardVector (Variables|/Game/DeadInside/BasePlayer/BP_BasePlayer.BP_BasePlayer_C|GetCamera (Variables|Character|GetChar%20Ref))) 1e+03)) 1e+01 (Utilities|Array|MakeArray "ObjectTypeQuery7") false (Utilities|Array|MakeArray (Variables|Character|GetChar%20Ref)) "None"))
    (if _returnvalue
      (for _array_element (Variables|Inventory|GetInteractablesInRange)
        (if (== (.HitActor (Collision|BreakHitResult _outhit)) _array_element)
          (Variables|Inventory|SetCurrent%20Interactable (.HitActor (Collision|BreakHitResult _outhit))))))))

(event EventBeginPlay
  (bind _returnvalue (Game|GetPlayerCameraManager 0))
  (bind _self self)
  ;[1 1 1] Begin Play
  (Utilities|FlowControl|Sequence
    (:then_0
      ;[1 1 1] Initialize BP Character
      (bind _char_ref (Class|BPIPlayer|PlayerRef(Message) (Game|GetPlayerCharacter 0)))
      (Variables|Character|SetChar%20Ref _char_ref))
    (:then_1
      ;[1 1 1] Limit Mouse Look
      (Variables|/Script/Engine.PlayerCameraManager|SetViewPitchMax _returnvalue 1e+01)
      (Variables|/Script/Engine.PlayerCameraManager|SetViewPitchMin _returnvalue -5.0))
    (:then_2
      ;[1 1 1] Player HUD
      (bind _returnvalue_2 (UserInterface|CreateWidget "/Game/DeadInside/Widget/UI_PlayerHUD.UI_PlayerHUD_C"))
      (bind _output_get (Variables|Character|SetPlayer%20HUD _returnvalue_2))
      (UserInterface|Viewport|AddtoViewport _output_get 0))
    (:then_3
      (Input|SetInputModeGameOnly _self)
      (Input|EnableInput _self _self))))

(event Input|ActionEvents|InputActionInteraction
  (params (Key :type Key%20Structure :default "None"))
  ;[1 1 1] Interaction Logic
  (:Pressed
    (bind _current_interactable (Variables|Inventory|GetCurrent%20Interactable)
      (:then
        (bind _interact_ref (Class|BPIInteract|InteractableRef(Message) _current_interactable))
        (if (Utilities|Enum|Equal(Enum) (Utilities|Struct|BreakStruct_InteractInfo (Variables|/Game/DeadInside/Interactables/BP_BaseInteractables.BP_BaseInteractables_C|GetInteract%20Info _interact_ref)) "NewEnumerator0")
          (CallFunction|WeaponPickup _current_interactable)
          (elif (Utilities|Enum|Equal(Enum) (Utilities|Struct|BreakStruct_InteractInfo (Variables|/Game/DeadInside/Interactables/BP_BaseInteractables.BP_BaseInteractables_C|GetInteract%20Info _interact_ref)) "NewEnumerator1")
            (CallFunction|ShieldPickup _current_interactable)
            (elif (Utilities|Enum|Equal(Enum) (Utilities|Struct|BreakStruct_InteractInfo (Variables|/Game/DeadInside/Interactables/BP_BaseInteractables.BP_BaseInteractables_C|GetInteract%20Info _interact_ref)) "NewEnumerator2")
              (CallFunction|HealthPickup _current_interactable)
              (elif (Utilities|Enum|Equal(Enum) (Utilities|Struct|BreakStruct_InteractInfo (Variables|/Game/DeadInside/Interactables/BP_BaseInteractables.BP_BaseInteractables_C|GetInteract%20Info _interact_ref)) "NewEnumerator3")
                (CallFunction|PotionPickup _current_interactable))))))
      (:else))))

(event Input|ActionEvents|InputActionPrimaryAttack
  (params (Key :type Key%20Structure :default "None"))
  (:Pressed
    (CallFunction|BasicAttack)))

(event Input|ActionEvents|InputActionRoll/Dodge
  (params (Key :type Key%20Structure :default "None"))
  ;[1 1 1] Roll Input
  (:Pressed
    (CallFunction|Roll)
    (Variables|Boolean|SetbIsRMPlaying false)))

(event Input|ActionEvents|InputActionDistraction
  (params (Key :type Key%20Structure :default "None"))
  (bind _char_ref (Variables|Character|GetChar%20Ref))
  (bind _returnvalue (Transformation|GetActorLocation _char_ref))
  ;[1 1 1] Distraction
  (:Pressed
    (Audio|PlaySoundatLocation "/Game/Assets/Sounds/Weapons/A_Weapon_FireSwing04.A_Weapon_FireSwing04" _returnvalue "0, 0, 0" 1.0 1.0 0.0 0 0 0)
    (Class|AISenseHearing|ReportNoiseEvent _returnvalue 1.0 self 1e+03 "Noise")))

(event Input|ActionEvents|InputActionSprint
  (params (Key :type Key%20Structure :default "None"))
  (bind _char_ref (Variables|Character|GetChar%20Ref))
  ;[1 1 1] Sprint
  (:Pressed
    (Class|BPIPlayer|SetPlayerSpeed(Message) _char_ref 6e+02))
  (:Released
    (Class|BPIPlayer|SetPlayerSpeed(Message) _char_ref 3e+02)))

(event Input|ActionEvents|InputActionSecondaryAttack
  (params (Key :type Key%20Structure :default "None"))
  (:Pressed
    (Variables|Inventory|GetShield
      (:then
        (Variables|Boolean|SetbIsBlocking true))
      (:else)))
  (:Released
    (Variables|Boolean|SetbIsBlocking false)))

(event Input|ActionEvents|InputActionHeal
  (params (Key :type Key%20Structure :default "None"))
  (bind _playerinfo (Variables|Default|GetPlayerInfo))
  (bind (_maxhealth _currenthealth) (Utilities|Struct|BreakPlayerInfo _playerinfo))
  ;[1 1 1] Heal
  (:Pressed
    (if (and (> (Variables|Inventory|GetHealth%20Count) 0) (not (Variables|Default|GetbIsDrinking)))
      (if (< _currenthealth _maxhealth)
        (Variables|Default|SetbIsDrinking true)
        (Utilities|Heal)))))

(event Input|ActionEvents|InputActionPotion_Heal
  (params (Key :type Key%20Structure :default "None"))
  (bind _playerinfo (Variables|Default|GetPlayerInfo))
  (bind (_maxarmor _currentarmor) (Utilities|Struct|BreakPlayerInfo _playerinfo))
  (:Pressed
    (Development|PrintString "Start")
    (if (and (not (Variables|Default|GetbIsDrinking)) (> (Variables|Inventory|GetPotion%20Count) 0))
      (if (< _currentarmor _maxarmor)
        (Variables|Default|SetbIsDrinking true)
        (Development|PrintString "Hello")
        (Utilities|PotionHeal)))))

(event Input|AxisEvents|InputAxisMoveForward
  (params (AxisValue :type Float%20%28single-precision%29))
  ;[1 1 1] Movement logic
  (Pawn|Input|AddMovementInput (Pawn|GetControlledPawn) (Math|Vector|GetForwardVector (Variables|/Script/Engine.Character|GetCapsuleComponent (Variables|Character|GetChar%20Ref))) AxisValue false))

(event Input|AxisEvents|InputAxisMoveRight
  (params (AxisValue :type Float%20%28single-precision%29))
  ;[1 1 1] Movement logic
  (Pawn|Input|AddMovementInput (Pawn|GetControlledPawn) (Math|Vector|GetRightVector (Variables|/Script/Engine.Character|GetCapsuleComponent (Variables|Character|GetChar%20Ref))) AxisValue false))

(event Input|AxisEvents|InputAxisLookUp
  (params (AxisValue :type Float%20%28single-precision%29))
  ;[1 1 1] Mouse Controls
  (Class|PlayerController|AddPitchInput AxisValue))

(event Input|AxisEvents|InputAxisTurn
  (params (AxisValue :type Float%20%28single-precision%29))
  ;[1 1 1] Mouse Controls
  (Class|PlayerController|AddYawInput AxisValue))

(fn ConstructionScript)

(fn DamageDealt
  (params (Damage%20Received :type Float%20%28single-precision%29))
  (bind _playerinfo (Variables|Default|GetPlayerInfo))
  (bind _playerinfo_2 (Variables|Default|GetPlayerInfo))
  (bind _char_ref (Variables|Character|GetChar%20Ref))
  (bind _char_ref_2 (Variables|Character|GetChar%20Ref))
  (bind (_maxarmor _currentarmor) (Utilities|Struct|BreakPlayerInfo _playerinfo))
  (bind (_maxhealth _currenthealth) (Utilities|Struct|BreakPlayerInfo _playerinfo_2))
  (if (<= _currentarmor 0.0)
    (Utilities|Struct|SetmembersinPlayerInfo (Variables|Default|GetPlayerInfo) (Math|Float|Clamp(Float) (- _currenthealth Damage%20Received) 0.0 _maxhealth))
    (if (<= (Utilities|Struct|BreakPlayerInfo (Variables|Default|GetPlayerInfo)) 0.0)
      (Animation|StopAnimMontage _char_ref (Animation|GetCurrentMontage _char_ref :!class /Script/Engine.Character))
      (Variables|/Game/DeadInside/Character/BP_Player.BP_Player_C|SetbIsPlayerDead _char_ref_2 true)
      (Default|Death _char_ref_2))
    (else
      (Utilities|Struct|SetmembersinPlayerInfo (Variables|Default|GetPlayerInfo) (Math|Float|Clamp(Float) (- _currentarmor Damage%20Received) 0.0 _maxarmor)))))

(fn PCRef
  (return self))