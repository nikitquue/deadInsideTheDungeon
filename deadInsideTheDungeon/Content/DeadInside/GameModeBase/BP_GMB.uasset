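; BP_GMB is the game mode for DeadInside, handling ambient music, the opening fade and player spawn placement.
; On BeginPlay it starts a 2D creepy dungeon ambience through SetMusic, which can also stop it, and fades the camera in from full opacity.
; New players spawn at a PlayerStart looked up by name, using the options string minus its first character, so level-open options can choose the spawn point.
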(event EventHandleStartingNewPlayer
  (params (NewPlayer :type Player%20Controller%20Object%20Reference))
  (bind _optionsstring (Variables|Default|GetOptionsString))
  (Class|GameModeBase|RestartPlayeratPlayerStart NewPlayer (Class|GameModeBase|FindPlayerStart NewPlayer (Utilities|String|GetSubstring _optionsstring 1 (- (Utilities|String|Len _optionsstring) 1)))))

(event EventBeginPlay
  (Utilities|FlowControl|Sequence
    (:then_0
      (CallFunction|SetMusic true))
    (:then_1
      (CameraFades|StartCameraFade :self (Game|GetPlayerCameraManager 0) :FromAlpha 1.0 :Duration 1.0))))

(fn ConstructionScript)

(fn SetMusic
  (params (Play? :type Boolean))
  (if Play?
    (bind _returnvalue (Audio|CreateSound2D "/Game/Creative_part/Audio/166187__drminky__creepy-dungeon-ambience.166187__drminky__creepy-dungeon-ambience" 1.0 1.0 0.0 0))
    (bind _output_get (Variables|Default|SetMusic _returnvalue))
    (Audio|Components|Audio|Play _output_get 0.0)
    (else
      (Audio|Components|Audio|Stop (Variables|Default|GetMusic)))))