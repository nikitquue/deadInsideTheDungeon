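; BP_GoblinBaseTest is a goblin enemy that chases the player and attacks in melee.
; On BeginPlay it caches its AI controller, finds the first BP_Player after a delay, focuses it and loops AIMoveTo toward it.
; An AttackRange overlap repeats the attack montage until the player leaves.
; A separate Box overlap deals damage when CanHitR is set, then clears that flag, which this file never sets back.
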(event OnComponentBeginOverlap(Box)
  (params (OverlappedComponent :type Primitive%20Component%20Object%20Reference) (OtherActor :type Actor%20Object%20Reference) (OtherComp :type Primitive%20Component%20Object%20Reference) (OtherBodyIndex :type Integer) (bFromSweep :type Boolean) (SweepResult :type Hit%20Result%20Structure%20%28by%20ref%29))
  (if (and (== OtherActor (Variables|Default|GetMyEnemy)) (Variables|Default|GetCanHit_R))
    (Variables|Default|SetCanHit_R false)
    (Default|TakenDamage (Variables|Default|GetMyEnemy) 3e+01)))

(event OnComponentBeginOverlap(AttackRange)
  (params (OverlappedComponent :type Primitive%20Component%20Object%20Reference) (OtherActor :type Actor%20Object%20Reference) (OtherComp :type Primitive%20Component%20Object%20Reference) (OtherBodyIndex :type Integer) (bFromSweep :type Boolean) (SweepResult :type Hit%20Result%20Structure%20%28by%20ref%29))
  (if (and (== OtherActor (Variables|Default|GetMyEnemy)) (not (Variables|Default|GetisAtacking)))
    (Variables|Default|SetCanAttack true)
    (Variables|Default|SetisAtacking true :!label _label)
    (Animation|Montage|PlayMontage (Variables|Character|GetMesh) "/Game/DeadInside/AI/goblin/source/Atack_goblin_montage.Atack_goblin_montage"
      (:OnCompleted
        (Variables|Default|SetisAtacking false)
        (if (Variables|Default|GetCanAttack)
          (goto _label))))))

(event OnComponentEndOverlap(AttackRange)
  (params (OverlappedComponent :type Primitive%20Component%20Object%20Reference) (OtherActor :type Actor%20Object%20Reference) (OtherComp :type Primitive%20Component%20Object%20Reference) (OtherBodyIndex :type Integer))
  (if (and (== OtherActor (Variables|Default|GetMyEnemy)) (Variables|Default|GetCanAttack))
    (Variables|Default|SetCanAttack false)))

(event Custom|getenemy
  (Utilities|FlowControl|Delay 1.0)
  (bind _outactors (Actor|GetAllActorsOfClass "/Game/DeadInside/Character/BP_Player.BP_Player_C"))
  (Variables|Default|SetMyEnemy (Utilities|Array|Get(acopy) _outactors))
  (AI|SetFocus (Variables|Default|GetAI_Controller) (Variables|Default|GetMyEnemy)))

(event Custom|BaseMovement
  (Utilities|IsValid (Variables|Default|GetMyEnemy) :!label _label
    (:Is%20Valid
      (AI|AIMoveTo self "0, 0, 0" (Variables|Default|GetMyEnemy) 5e+01 false
        (:OnSuccess
          (Utilities|FlowControl|Delay 3.0)
          (goto _label))
        (:OnFail
          (goto _label))))
    (:Is%20Not%20Valid
      (Utilities|FlowControl|Delay 1.0)
      (goto _label))))

(event EventBeginPlay
  (Utilities|FlowControl|Sequence
    (:then_0
      (CallFunction|Getenemy))
    (:then_1
      (CallFunction|BaseMovement))
    (:then_2
      (bind _asaic_goblin_bp (Utilities|Casting|CastToAIC_Goblin_BP (Pawn|GetController)))
      (Variables|Default|SetAI_Controller _asaic_goblin_bp))))

(fn ConstructionScript)

(fn EnemyRef
  (return 0))